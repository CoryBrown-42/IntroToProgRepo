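; Pickup actor whose appearance and value depend on its Type enum, with variants such as Ultra Jump and Slow Mo.
; The construction script uses the enum name as a data table row key and passes the found row to SetProperty, which applies mesh, material and Value.
; An older hard-coded switch for the same properties remains disconnected and never runs.
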(fn ConstructionScript
  (bind _returnvalue (Utilities|GetDataTableRow "/Game/Poly/NewDataTable.NewDataTable" (Utilities|String|StringToName (Utilities|String|EnumtoString (Variables|Default|GetType))))
    (:then
      (CallFunction|SetProperty _returnvalue))))

(fn SetProperty
  (params (PickUp :type Pick%20Up%20Structure%20%28by%20ref%29))
  (bind (_name _mesh _material _value) (Utilities|Struct|BreakPickUp PickUp))
  (bind _polymesh (Variables|Default|GetPolyMesh))
  (Components|StaticMesh|SetStaticMesh _polymesh _mesh)
  (Rendering|Material|SetMaterial _polymesh 0 _material)
  (Variables|Default|SetValue _value))