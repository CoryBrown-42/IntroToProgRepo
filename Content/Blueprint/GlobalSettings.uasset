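; GlobalSettings is a Blueprint that drives a day/night cycle by rotating a directional light on a timer.
; Each tick of the timer, which loops when DayNight is set, updates the sky sphere and writes the sun direction to the GlobalMaterialSettings parameter collection.
; The light's pitch sign toggles fog visibility and an AO override parameter.
; Discord presence and Twitch chat code remains but is disconnected.
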(event OnChatCommandEntered(TwitchActor)
  (params (message :type String) (data :type Chat%20Message%20Data%20Structure)))

(event Custom|SetSunRotation
  (bind _fog (Variables|Default|GetFog))
  (bind _component (Variables|/Script/Engine.ExponentialHeightFog|GetComponent _fog))
  (bind _light (Variables|Default|GetLight)
    (:then
      (bind _skysphere (Variables|Default|GetSkySphere)
        (:then
          (Transformation|AddWorldRotation (Variables|/Script/Engine.Light|GetLightComponent _light) "0.100000, 0, 0" false false)
          (Default|UpdateSunDirection _skysphere)
          (Rendering|Material|SetVectorParameterValue "/Game/Materials/GlobalMaterialSettings.GlobalMaterialSettings" "SunDirection" (Math|Conversions|ToLinearColor(Vector) (Math|Vector|GetForwardVector (Variables|/Script/Engine.Light|GetLightComponent _light))) :!class /Script/Engine.KismetMaterialLibrary)
          (if (< (.pitch (Transformation|GetWorldRotation (Variables|/Script/Engine.Light|GetLightComponent _light))) 0.0)
            (Rendering|Material|SetScalarParameterValue "/Game/Materials/GlobalMaterialSettings.GlobalMaterialSettings" "AO_Override" 1.0 :!class /Script/Engine.KismetMaterialLibrary)
            (Rendering|SetVisibility _component true false)
            (else
              (Rendering|Material|SetScalarParameterValue "/Game/Materials/GlobalMaterialSettings.GlobalMaterialSettings" "AO_Override" 0.0 :!class /Script/Engine.KismetMaterialLibrary)
              (Rendering|SetVisibility _component false false))))
        (:else)))
    (:else)))

(event Custom|OnStateSetEvent
  (params (StateSetResult :type EDiscordReturnResult%20Enum :default "Ok"))
  (switch Utilities|FlowControl|Switch|SwitchonEDiscordReturnResult StateSetResult))

(event Custom|OnDetailsSet_Event
  (params (StateSetResult :type EDiscordReturnResult%20Enum :default "Ok"))
  (switch Utilities|FlowControl|Switch|SwitchonEDiscordReturnResult StateSetResult))

(event EventBeginPlay
  (Utilities|Time|SetTimerbyEvent (delegate Custom|SetSunRotation) (Variables|Default|GetRate) (Variables|Default|GetDay&Night)))

(fn ConstructionScript)