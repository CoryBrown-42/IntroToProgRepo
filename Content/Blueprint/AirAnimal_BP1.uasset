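; AirAnimal_BP1 is an animal character that takes flight when another Character enters its TooClose trigger.
; The overlap switches its movement to Flying and adds a single movement input along fixed world forward and up, regardless of where the intruder is.
; A looping BeginPlay timer fires MoveToRandomLocation, but that event is empty.
; The AI random-wander move with result printing is disconnected and never runs.
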(event OnComponentBeginOverlap(TooClose)
  (params (OverlappedComponent :type Primitive%20Component%20Object%20Reference) (OtherActor :type Actor%20Object%20Reference) (OtherComp :type Primitive%20Component%20Object%20Reference) (OtherBodyIndex :type Integer) (bFromSweep :type Boolean) (SweepResult :type Hit%20Result%20Structure%20%28by%20ref%29))
  (bind _charactermovement (Variables|Character|GetCharacterMovement))
  (Utilities|Casting|CastToCharacter OtherActor)
  (Pawn|Components|CharacterMovement|SetMovementMode _charactermovement "MOVE_Flying" 0)
  (Pawn|Input|AddMovementInput (+ (* (Class|KismetMathLibrary|VectorForward) 1e+03) (* (Math|Vector|VectorUp) 1e+03)) (Variables|/Script/Engine.CharacterMovementComponent|GetMaxFlySpeed _charactermovement) false))

(event Custom|MoveToRandomLocation)

(event EventBeginPlay
  (Utilities|Time|SetTimerbyEvent (delegate Custom|MoveToRandomLocation) 5.0 true))

(fn ConstructionScript)