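; Pickup actor that flies into the player's backpack when picked up and adds health.
; Construction and BeginPlay read a data table row keyed by the Type enum to set mesh, material, value and name label.
; PickupItem disables collision, then a timeline shrinks, spins and moves it toward the backpack before destroying it and playing the player's backpack effect.
; FindPlayer turns the name widget toward the camera, but its looping timer is unconnected.
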(event Custom|FindPlayer
  (bind _widget (Variables|Default|GetWidget))
  ;[1 1 1] Look at player
  (Transformation|SetWorldRotation (Variables|Default|GetWidget) (Math|Interpolation|RInterpTo (Transformation|GetWorldRotation _widget) (Math|Rotator|FindLookatRotation (Transformation|GetWorldLocation _widget) (Transformation|GetWorldLocation (Variables|/Script/Engine.PlayerCameraManager|GetTransformComponent (Game|GetPlayerCameraManager 0)))) 0.5 5.0) false false))

(event EventBeginPlay
  ;[0.5341 0.4775 1] On Begin play - get data table row and set property
  (bind _returnvalue (Utilities|GetDataTableRow "/Game/Item/PickupTable.PickupTable" (Utilities|String|StringToName (Utilities|String|EnumtoString (Variables|Item|GetType))))
    (:then
      (CallFunction|SetProperty _returnvalue))))

(event EventPickupItem
  (params (Player :type Third%20Person%20Character%20Soft%20Object%20Reference))
  ;[1 0.9375 0.2977] Animate going into backpack
  (Variables|Default|SetPlayer Player)
  (Utilities|PreparePickupforAnimation)
  (bind _lerp_alpha (Timeline|Animate PlayFromStart)
    (:Update
      (CallFunction|PickupAnimation _lerp_alpha (Variables|Default|GetPlayer)))
    (:Finished
      (Actor|DestroyActor)
      (Default|PlayBackpackEffect (Utilities|ResolveSoftReference (Variables|Default|GetPlayer)) "/Game/StarterContent/Particles/P_Explosion.P_Explosion" "/Game/StarterContent/Audio/Explosion_Cue.Explosion_Cue")
      (Utilities|AddHealth 1))))

(fn ConstructionScript
  (bind _returnvalue (Utilities|GetDataTableRow "/Game/Item/PickupTable.PickupTable" (Utilities|String|StringToName (Utilities|String|EnumtoString (Variables|Item|GetType))))
    (:then
      (CallFunction|SetProperty _returnvalue))))

(fn SetProperty
  (params (PickUp :type Pick%20Up%20Structure%20%28by%20ref%29))
  (bind (_name _mesh _material _value) (Utilities|Struct|BreakPickUp PickUp))
  (bind _polymesh (Variables|Default|GetPolyMesh))
  (Components|StaticMesh|SetStaticMesh _polymesh _mesh)
  (Rendering|Material|SetMaterial _polymesh 0 _material)
  (Variables|Item|SetValue _value)
  (Rendering|Components|TextRender|SetText (Variables|Default|GetName) (Utilities|Text|ToText(String) _name))
  ;[0.3095 0.8698 1] Change the name of the widget to name of pickup
  (bind _asname (Utilities|Casting|CastToName (UserInterface|GetUserWidgetObject (Variables|Default|GetWidget))))
  (Variables|/Game/Item/Name.Name_C|SetName _asname _name))

(fn PickupAnimation
  (params (LerpAlpha :type Float%20%28single-precision%29) (Player :type Third%20Person%20Character%20Soft%20Object%20Reference))
  (bind _returnvalue (* 1e+02 LerpAlpha))
  (Utilities|FlowControl|Sequence
    (:then_0
      (Transformation|SetWorldScale3D (Variables|Default|GetPolyMesh) (Math|Vector|Lerp(Vector) "1.000000,1.000000,1.000000" "0.100000,0.100000,0.100000" LerpAlpha)))
    (:then_1
      (Transformation|SetActorLocation (Math|Vector|Lerp(Vector) (Variables|Default|GetOriginalLocation) (- (Transformation|GetWorldLocation (Variables|/Game/Blueprint/ThirdPersonCharacter.ThirdPersonCharacter_C|GetBackpack (Utilities|ResolveSoftReference Player))) "0, 0,100.000000") LerpAlpha) false false))
    (:then_2
      (Transformation|AddWorldRotation (Variables|Default|GetPolyMesh) (Math|Rotator|MakeRotator _returnvalue _returnvalue _returnvalue) false false))))